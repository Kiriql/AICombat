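; GA_EquipWeapon is a Gameplay Ability that equips or unequips a weapon on the avatar actor through its BP_WeaponsManagerComponent.
; Activated by a gameplay event, it commits, then switches on the first target tag to equip the axe or staff, or unequip for any other tag.
; Only the two equip branches end the ability; the unequip branch and a missing component leave it active.
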(event Ability|EventActivateAbilityFromEvent
  (params (EventData :type Gameplay%20Event%20Data%20Structure%20%28by%20ref%29))
  (bind _returnvalue (Ability|GetAvatarActorfromActorInfo))
  (bind _returnvalue_2 (Actor|GetComponentbyClass _returnvalue "/Game/Weapons/BP_WeaponsManagerComponent.BP_WeaponsManagerComponent_C"))
  (Ability|CommitAbility)
  (Utilities|IsValid _returnvalue_2
    (:Is%20Valid
      (|SwitchGameplayTag (Utilities|Array|Get(acopy) (GameplayTags|BreakGameplayTagContainer (.TargetTags (Utilities|Struct|BreakGameplayEventData EventData))))
        (:Default
          (Default|UnequipWeapon _returnvalue_2))
        (:Weapon.Melee.Axe
          (Default|EquipWeapon _returnvalue_2 "/Game/Weapons/BP_Weapon_Axe.BP_Weapon_Axe_C")
          (Ability|EndAbility))
        (:Weapon.Ranged.Staff
          (Default|EquipWeapon _returnvalue_2 "/Game/Weapons/BP_Weapon_Staff.BP_Weapon_Staff_C")
          (Ability|EndAbility))))))