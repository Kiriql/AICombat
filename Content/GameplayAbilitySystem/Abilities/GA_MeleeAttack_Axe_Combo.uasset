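; Axe combo melee Gameplay Ability that extends a parent melee attack, letting timed input continue the attack chain with rising damage.
; On montage start it resets the combo count and listens for gameplay events marking window start, window end and input.
; At window end, input received inside the window increments the count; otherwise the ability ends.
; Each hit scan scales damage by combo count before calling the parent handler.
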(event Ability|EventActivateAbility
  (|CallParentFunction) ; This node is disabled and will not be called.\nDrag off pins to build functionality.
)

(event Ability|EventOnEndAbility
  (params (bWasCancelled :type Boolean))
  (|CallParentFunction bWasCancelled) ; This node is disabled and will not be called.\nDrag off pins to build functionality.
)

(event EventMontageStarted
  (Development|PrintString (Utilities|String|Append "ABILITY START Authority:" (Utilities|String|ToString(Boolean) (Ability|HasAuthority (Ability|GetAvatarActorfromActorInfo)))))
  (Variables|Default|SetComboCount 1)
  (Ability|Tasks|WaitGameplayEvent "(TagName=\"Event.ContinueCombo.Start\")" 0
    (:then
      (Ability|Tasks|WaitGameplayEvent "(TagName=\"Event.ContinueCombo.End\")" 0
        (:then
          (Ability|Tasks|WaitGameplayEvent "(TagName=\"Event.ContinueCombo.Input\")" 0
            (:EventReceived
              (Variables|Default|SetbReceivedInputInAtRightTime (Variables|Default|GetbIsWithinComboWindow)))))
        (:EventReceived
          (Variables|Default|SetbIsWithinComboWindow false)
          (if (Variables|Default|GetbReceivedInputInAtRightTime)
            (Math|Integer|IncrementInt (Variables|Default|GetComboCount))
            (else
              (Ability|EndAbility))))))
    (:EventReceived
      (Development|PrintString (Utilities|String|Append "EVENT 1 Combo:" (Utilities|String|ToString(Integer) (Variables|Default|GetComboCount))))
      (Variables|Default|SetbIsWithinComboWindow true)
      (Variables|Default|SetbReceivedInputInAtRightTime false))))

(event EventHandleHitScanStart
  (Variables|Default|SetDamageMagnitude (* -25.0 (Variables|Default|GetComboCount)))
  (|CallParentFunction))