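; Actor component that manages equipping and unequipping weapons on an ArenaCharacterBase owner.
; On the authority, EquipWeapon spawns and socket-attaches the weapon and grants its configured abilities; requesting the same class unequips it, another class swaps.
; Unequipping destroys the weapon and removes those abilities.
; Anim class and movement settings follow the weapon or unarmed config, and are reapplied through OnRep_EquippedWeapon.
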(event Custom|UnequipWeapon
  (bind _equippedweapon (Variables|Default|GetEquippedWeapon)
    (:then
      (Actor|DestroyActor _equippedweapon)
      (Class|ArenaCharacterBase|RemoveAbilities (Variables|Default|GetOwningCharacter) (Variables|Default|GetAbilitiesGrantedByWeapon))
      (Variables|Default|SetEquippedWeapon 0)
      (CallFunction|SetUnarmedWeaponProperties))
    (:else)))

(event Custom|EquipWeapon
  (params (WeaponClass :type BP%20Weapon%20Base%20Class%20Reference))
  (Development|PrintString (Utilities|String|Append "Start" ": " (Utilities|GetClassDisplayName WeaponClass)))
  (Networking|SwitchHasAuthority
    (:Authority
      (Variables|Default|GetOwningCharacter
        (:then
          (bind _equippedweapon (Variables|Default|GetEquippedWeapon)
            (:then
              (if (== (Utilities|GetClass _equippedweapon) WeaponClass)
                (CallFunction|UnequipWeapon)
                (else
                  (CallFunction|UnequipWeapon)
                  (bind _returnvalue (Game|SpawnActorfromClass WeaponClass (Math|Transform|MakeTransform "0, 0, 0" "0, 0, 0" "1.000000,1.000000,1.000000") "Undefined" "MultiplyWithRoot" 0 (Variables|Default|GetOwningCharacter) :!label _label))
                  (bind _output_get (Variables|Default|SetEquippedWeapon _returnvalue))
                  (Transformation|AttachComponentToComponent _output_get (Variables|/Script/Engine.Character|GetMesh (Variables|Default|GetOwningCharacter)) (.EquippedSocketName (Utilities|Struct|BreakS_WeaponConfig (Variables|/Game/Weapons/BP_Weapon_Base.BP_Weapon_Base_C|GetWeaponConfig _output_get))) "SnapToTarget" "SnapToTarget" "SnapToTarget" true)
                  (bind _returnvalue_2 (Class|ArenaCharacterBase|GrantAbilities (Variables|Default|GetOwningCharacter) (Utilities|Struct|BreakS_WeaponConfig (Variables|/Game/Weapons/BP_Weapon_Base.BP_Weapon_Base_C|GetWeaponConfig (Variables|Default|GetEquippedWeapon)))))
                  (Variables|Default|SetAbilitiesGrantedByWeapon _returnvalue_2)
                  (CallFunction|SetEquippedWeaponProperties))))
            (:else
              (goto _label))))
        (:else)))))

(event Custom|SetEquippedWeaponProperties
  (bind _owningcharacter (Variables|Default|GetOwningCharacter))
  (bind _charactermovement (Variables|/Script/Engine.Character|GetCharacterMovement _owningcharacter))
  (bind _equippedweapon (Variables|Default|GetEquippedWeapon)
    (:then
      (Components|SkeletalMesh|SetAnimInstanceClass (Variables|/Script/Engine.Character|GetMesh (Variables|Default|GetOwningCharacter)) (.AnimClass (Utilities|Struct|BreakS_WeaponConfig (Variables|/Game/Weapons/BP_Weapon_Base.BP_Weapon_Base_C|GetWeaponConfig _equippedweapon))))
      (Variables|/Script/Engine.CharacterMovementComponent|SetMaxWalkSpeed _charactermovement (.MaxWalkSpeed (Utilities|Struct|BreakS_MovementProperties (.MovementProperties (Utilities|Struct|BreakS_WeaponConfig (Variables|/Game/Weapons/BP_Weapon_Base.BP_Weapon_Base_C|GetWeaponConfig _equippedweapon))))))
      (Variables|/Script/Engine.CharacterMovementComponent|SetbOrientRotationToMovement _charactermovement (.bOrientRotationToMovement (Utilities|Struct|BreakS_MovementProperties (.MovementProperties (Utilities|Struct|BreakS_WeaponConfig (Variables|/Game/Weapons/BP_Weapon_Base.BP_Weapon_Base_C|GetWeaponConfig _equippedweapon))))))
      (Variables|/Script/Engine.CharacterMovementComponent|SetbUseControllerDesiredRotation _charactermovement (.bUseControllerDesiredRotation (Utilities|Struct|BreakS_MovementProperties (.MovementProperties (Utilities|Struct|BreakS_WeaponConfig (Variables|/Game/Weapons/BP_Weapon_Base.BP_Weapon_Base_C|GetWeaponConfig _equippedweapon)))))))
    (:else)))

(event Custom|SetUnarmedWeaponProperties
  (bind _owningcharacter (Variables|Default|GetOwningCharacter))
  (bind _unarmedweaponconfig (Variables|Default|GetUnarmedWeaponConfig))
  (bind (_abilitiestogrant _equippedsocketname _stowedsocketname _animclass _equipmontage _unequipmontage _movementproperties) (Utilities|Struct|BreakS_WeaponConfig _unarmedweaponconfig))
  (bind _charactermovement (Variables|/Script/Engine.Character|GetCharacterMovement _owningcharacter))
  (bind (_maxwalkspeed _borientrotationtomovement _busecontrollerdesiredrotation) (Utilities|Struct|BreakS_MovementProperties _movementproperties))
  (Components|SkeletalMesh|SetAnimInstanceClass (Variables|/Script/Engine.Character|GetMesh (Variables|Default|GetOwningCharacter)) _animclass)
  (Variables|/Script/Engine.CharacterMovementComponent|SetMaxWalkSpeed _charactermovement _maxwalkspeed)
  (Variables|/Script/Engine.CharacterMovementComponent|SetbOrientRotationToMovement _charactermovement _borientrotationtomovement)
  (Variables|/Script/Engine.CharacterMovementComponent|SetbUseControllerDesiredRotation _charactermovement _busecontrollerdesiredrotation))

(event EventBeginPlay
  (bind _asarena_character_base (Utilities|Casting|CastToArenaCharacterBase (Components|GetOwner)))
  (Variables|Default|SetOwningCharacter _asarena_character_base))

(fn OnRepEquippedWeapon
  (Variables|Default|GetEquippedWeapon
    (:then
      (CallFunction|SetEquippedWeaponProperties))
    (:else
      (CallFunction|SetUnarmedWeaponProperties))))